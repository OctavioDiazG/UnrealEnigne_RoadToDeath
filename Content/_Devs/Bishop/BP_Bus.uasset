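; BP_Bus is an actor that periodically spawns BP_Obstacle actors ahead of the actor it is attached to.
; Tick accumulates a timer, and once it exceeds SpawnRate it resets and prints a debug "Spawn" message.
; Each obstacle spawns relative to the attach parent's location, at a fixed world X and Z offset with a random Y offset for lateral spread.
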(event `self.ReceiveTick`
  (params (DeltaSeconds :type "Float (single-precision)"))
  (set `self.SpawnTime` (+ (`self.SpawnTime`) DeltaSeconds))
  (if (> (`self.SpawnTime`) (`self.SpawnRate`))
    (set `self.SpawnTime` 0.0)
    (`KismetSystemLibrary.PrintString` "Spawn")
    (`|SpawnActorFromClass` "/Game/_Devs/Bishop/BP_Obstacle.BP_Obstacle_C" (`KismetMathLibrary.Conv_VectorToTransform` (+ (`self.K2_GetActorLocation` (`self.GetAttachParentActor`)) (`KismetMathLibrary.MakeVector` 7500.0 (`KismetMathLibrary.RandomFloatInRange` -360.0 360.0) 150.0))) "Undefined" "OverrideRootScale" null null)))

(fn `UserConstructionScript`)