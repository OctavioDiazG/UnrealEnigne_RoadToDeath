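; BP_Ghost is a ghost actor that creeps along the world X axis while the player is not watching.
; Each moving Tick adds GhostVelocity to X without delta-time scaling.
; If the first-person character's PlayerIsWatching flag is set, the ghost snaps to the X position of BP_Bus's Arrow and stops.
; While stopped, a Delay loop periodically randomizes IsMoving to decide when it moves again.
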(event `self.ReceiveBeginPlay`
  (bind _asbp_first_person_character (cast `/Game/FirstPerson/Blueprints/BP_FirstPersonCharacter` (`GameplayStatics.GetPlayerCharacter` 0)))
  (set `self.Player` _asbp_first_person_character)
  (bind _returnvalue (`GameplayStatics.GetActorOfClass` "/Game/_Devs/Bishop/BP_Bus.BP_Bus_C"))
  (set `self.Bus` _returnvalue))

(event `self.ReceiveTick`
  (params (DeltaSeconds :type "Float (single-precision)"))
  (bind (_returnvalue_x _returnvalue_y _returnvalue_z) (`KismetMathLibrary.BreakVector` (`self.K2_GetActorLocation`)))
  (bind (_returnvalue_x_2 _returnvalue_y_2 _returnvalue_z_2) (`KismetMathLibrary.BreakVector` (`self.K2_GetActorLocation`)))
  (bind _returnvalue_x_3 (`KismetMathLibrary.BreakVector` (`SceneComponent.K2_GetComponentLocation` (`/Game/_Devs/Bishop/BP_Bus.Arrow` (`self.Bus`)))))
  (if (`self.IsMoving`) :!label _label
    (if (`/Game/FirstPerson/Blueprints/BP_FirstPersonCharacter.PlayerIsWatching` (`self.Player`))
      (`self.K2_SetActorLocation` (`KismetMathLibrary.MakeVector` _returnvalue_x_3 _returnvalue_y _returnvalue_z))
      (set `self.IsMoving` false)
      (else
        (`self.K2_SetActorLocation` (`KismetMathLibrary.MakeVector` (+ _returnvalue_x_2 (`self.GhostVelocity`)) _returnvalue_y_2 _returnvalue_z_2))))
    (else
      (`KismetSystemLibrary.Delay` 5.0)
      (set `self.IsMoving` (`KismetMathLibrary.RandomBool`))
      (goto _label))))

(fn `UserConstructionScript`)