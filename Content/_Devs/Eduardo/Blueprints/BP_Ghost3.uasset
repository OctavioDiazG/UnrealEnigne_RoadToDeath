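; BP_Ghost3 is a ghost enemy that switches with the lights and kills the player on contact.
; OnLightsOff sets IsActive and OnLightson clears it, while the active behavior on Tick is only a placeholder debug print.
; Overlapping the collision component destroys BP_FirstPersonCharacter, shows the mouse cursor and displays WBP_DeathScreen.
; The overlap kill does not check IsActive, so it also applies while the ghost is inactive.
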(event `self.ReceiveTick`
  (params (DeltaSeconds :type "Float (single-precision)"))
  (if (`self.isActive?`)
    ;[1 1 1] Funcionalidad del fantasma
    (`KismetSystemLibrary.PrintString` "Ghost Active")))

(event `/Game/_Devs/Eduardo/Interfaces/BPI_LightSystem.OnLightsOn`
  ;[1 1 1] Desactivate Ghost
  (set `self.isActive?` false))

(event `/Game/_Devs/Eduardo/Interfaces/BPI_LightSystem.OnLightsOff`
  ;[1 1 1] Activate Ghost
  (set `self.isActive?` true))

(event `self.CollisionComponent.OnComponentBeginOverlap`
  (params (OverlappedComponent :type "PrimitiveComponent Object Reference") (OtherActor :type "Actor Object Reference") (OtherComp :type "PrimitiveComponent Object Reference") (OtherBodyIndex :type Integer) (bFromSweep :type Boolean) (SweepResult :type "HitResult Structure (by ref)"))
  (bind _asbp_first_person_character (cast `/Game/FirstPerson/Blueprints/BP_FirstPersonCharacter` OtherActor))
  (`self.K2_DestroyActor` _asbp_first_person_character)
  (set `PlayerController.bShowMouseCursor` true (`GameplayStatics.GetPlayerController` 0))
  (bind _returnvalue (`|GenericCreateObject` "/Game/_Devs/Eduardo/UI_Widgets/WBP_DeathScreen.WBP_DeathScreen_C"))
  (`UserWidget.AddToViewport` _returnvalue 0))

(fn `UserConstructionScript`)