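; BP_PlayerMenu is a menu player actor that turns its camera for settings and moves into the palace on play.
; BeginPlay shows the mouse cursor.
; Tick polls a Settings flag to play or reverse the Rot timeline, which yaws the camera half a turn.
; Play_Event runs the Move timeline, lerping the actor's X from its current position toward a fixed target.
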(event `self.ReceiveBeginPlay`
  ;[1 0.7812 0] Show Mouse Cursor
  (set `PlayerController.bShowMouseCursor` true (`GameplayStatics.GetPlayerController` 0)))

(event `self.ReceiveTick`
  (params (DeltaSeconds :type "Float (single-precision)"))
  ;[0.7708 0 0.06206] If settings is pressed then rotate camera
  (if (`self.Settings`)
    (bind (_direction _rotar) (`Timeline|Rot` :!label _label)
      (:`Update`
        (`SceneComponent.K2_SetRelativeRotation` (`self.Camera`) (`KismetMathLibrary.MakeRotator` 0.0 0.0 (`KismetMathLibrary.Lerp` 0.0 -180.0 _rotar)) false false)))
    (else
      (goto _label :!via `Reverse`))))

(event `Play_Event`
  (bind (_returnvalue_x _returnvalue_y _returnvalue_z) (`KismetMathLibrary.BreakVector` (`self.K2_GetActorLocation`)))
  ;[1 0.7812 0] If play button is pressed then move player into the palace
  (bind (_direction _move) (`Timeline|Move`)
    (:`Update`
      (`self.K2_SetActorLocation` (`KismetMathLibrary.MakeVector` (`KismetMathLibrary.Lerp` _returnvalue_x 20000.0 _move) _returnvalue_y _returnvalue_z)))))

(fn `UserConstructionScript`)